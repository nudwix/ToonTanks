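; Game mode for Toon Tanks that drives the match's UI from the start screen to the return to the main menu.
; StartGame shows a start widget, then adds the HUD after a delay, and Tick refreshes its enemy count from TargetTowers every frame.
; GameOver shows a victory or defeat message, then after a short delay removes the HUD and opens the MainMenu level.
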(event EventTick
  (params (DeltaSeconds :type Float%20%28single-precision%29))
  (Rendering|Components|TextRender|SetText (Variables|/Game/Blueprints/Widgets/Game/WBP_InterfaceWidget.WBP_InterfaceWidget_C|GetEnemyNumText (stale EventStartGame _returnvalue_2)) (Utilities|Text|ToText(Integer) (Variables|Default|GetTargetTowers))))

(event EventStartGame
  (bind _returnvalue (UserInterface|CreateWidget "/Game/Blueprints/Widgets/Game/WBP_StartGameWidget.WBP_StartGameWidget_C"))
  (UserInterface|Viewport|AddtoViewport _returnvalue 0)
  (bind _returnvalue_2 (UserInterface|CreateWidget "/Game/Blueprints/Widgets/Game/WBP_InterfaceWidget.WBP_InterfaceWidget_C"))
  (Utilities|FlowControl|Delay 4.0)
  (UserInterface|Viewport|AddtoViewport _returnvalue_2 0))

(event EventGameOver
  (params (bWonGame :type Boolean))
  (bind _returnvalue (UserInterface|CreateWidget "/Game/Blueprints/Widgets/Game/WBP_GameOverWidget.WBP_GameOverWidget_C"))
  (Rendering|Components|TextRender|SetText (Variables|/Game/Blueprints/Widgets/Game/WBP_GameOverWidget.WBP_GameOverWidget_C|GetDisplayText _returnvalue) (select bWonGame "Victory!" "Game Over!"))
  (UserInterface|Viewport|AddtoViewport _returnvalue 0)
  (Utilities|FlowControl|Delay 2.0)
  (Widget|RemovefromParent (stale EventStartGame _returnvalue_2))
  (Game|OpenLevel(byName) "MainMenu"))

(fn ConstructionScript)